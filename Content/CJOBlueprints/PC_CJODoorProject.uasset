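; Player controller for the CJO door project that toggles a pause menu from the Pause input action.
; Opening creates the CJO_MainMenuHUD widget, shows the cursor, allows UI input, pauses the game and hides the FirstPersonCharacter's HUD.
; Closing removes the widget and reverses those changes, using the stored widget reference's validity as the open/closed state.
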(event `InputAction|Pause`
  (params (Key :type "Key Structure"))
  (bind _returnvalue (`GameplayStatics.GetPlayerController` 0))
  (bind _returnvalue_2 (`GameplayStatics.GetPlayerController` 0))
  ;[1 1 1] Pause Menu
  (:`Pressed`
    (`/Engine/EditorBlueprintResources/StandardMacros.IsValid` (`self.PauseUIRef`)
      (:`Is Valid`
        (`Widget.RemoveFromParent` (`self.PauseUIRef`))
        (set `self.PauseUIRef` null)
        (`WidgetBlueprintLibrary.SetInputMode_GameOnly` _returnvalue)
        (set `PlayerController.bShowMouseCursor` false _returnvalue)
        (`GameplayStatics.SetGamePaused` false)
        (`/Game/FirstPersonBP/Blueprints/FirstPersonCharacter.TogglehudON` (cast `/Game/FirstPersonBP/Blueprints/FirstPersonCharacter` (`GameplayStatics.GetPlayerCharacter` 0) :!pure true)))
      (:`Is Not Valid`
        (bind _returnvalue_3 (`|CreateWidget` "/Game/CJOBlueprints/CJO_MainMenuHUD.CJO_MainMenuHUD_C"))
        (bind _output_get (set `self.PauseUIRef` _returnvalue_3))
        (`UserWidget.AddToViewport` _output_get 0)
        (`WidgetBlueprintLibrary.SetInputMode_GameAndUIEx` _returnvalue_2 null)
        (set `PlayerController.bShowMouseCursor` true _returnvalue_2)
        (`GameplayStatics.SetGamePaused` true)
        (`/Game/FirstPersonBP/Blueprints/FirstPersonCharacter.TogglehudOFF` (cast `/Game/FirstPersonBP/Blueprints/FirstPersonCharacter` (`GameplayStatics.GetPlayerCharacter` 0) :!pure true))))))

(fn `UserConstructionScript`)